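; BP_SlowZone is an interactable zone that slows overlapping actors through the Gameplay Ability System.
; On begin overlap it calls the parent, applies GE_Slow to the actor's Ability System Component and stores the returned handle.
; On end overlap it removes one stack using that handle, which is a single variable overwritten by each new overlap.
; An alternative removal by source effect is left unconnected.
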(event Collision|EventActorEndOverlap
  (params (OtherActor :type Actor%20Object%20Reference))
  (GameplayEffects|RemoveActiveGameplayEffect (Ability|GetAbilitySystemComponent OtherActor) (Variables|Default|GetGE_Slow_Handle) 1))

(event Collision|EventActorBeginOverlap
  (params (OtherActor :type Actor%20Object%20Reference))
  (|CallParentFunction OtherActor)
  (bind _returnvalue (GameplayEffects|ApplyGameplayEffectToSelf :self (Ability|GetAbilitySystemComponent OtherActor) :GameplayEffectClass "/Game/GAS/GameplayEffects/GE_Slow.GE_Slow_C" :Level 1.0))
  (Variables|Default|SetGE_Slow_Handle _returnvalue))

(fn ConstructionScript
  (|CallParentFunction))